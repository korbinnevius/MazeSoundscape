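; SoundManager is an actor that plays a Bells sound on a left mouse click and tracks its distance to the player character.
; The click handler itself calls EnableInput for the first player controller before starting the sound.
; BeginPlay stores the starting distance as MaxVariableDistance, and Tick prints the current distance normalized against it as debug text, without feeding it to the audio.
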(event Collision|EventActorBeginOverlap
  (params (OtherActor :type Actor%20Object%20Reference)))

(event EventBeginPlay
  (Utilities|FlowControl|DoOnce false
    (:Completed
      (Variables|Default|SetMaxVariableDistance (Transformation|GetDistanceTo (Game|GetPlayerCharacter 0))))))

(event EventTick
  (params (DeltaSeconds :type Float%20%28single-precision%29))
  (Development|PrintString (Utilities|String|ToString(Float) (Math|Float|NormalizetoRange (Transformation|GetDistanceTo (Game|GetPlayerCharacter 0)) 0.0 (Variables|Default|GetMaxVariableDistance)))))

(event Input|MouseEvents|LeftMouseButton
  (params (Key :type Key%20Structure :default "None"))
  (:Pressed
    (Input|EnableInput (Game|GetPlayerController 0))
    (Audio|Components|Audio|Play (Variables|Default|GetBells) 0.0)))

(fn ConstructionScript)